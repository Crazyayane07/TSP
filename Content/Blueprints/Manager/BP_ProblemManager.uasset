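; BP_ProblemManager is a manager Blueprint that generates a randomized layout of BP_City actors.
; SetUpCities destroys and clears the existing Cities, then spawns NumberOfCities new ones, each named by its index and stored in that array.
; Each city lands at a random X/Y within symmetric bounds around the world origin, at a configurable fixed height.
; The event graph and construction script are empty, so nothing in this Blueprint calls SetUpCities.
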(fn `SetUpCities`
  (bind _maxrandomx (`self.MaxRandomX`))
  (bind _maxrandomy (`self.MaxRandomY`))
  (for _array_element (`self.Cities`)
    (`self.K2_DestroyActor` _array_element))
  (`KismetArrayLibrary.Array_Clear` (`self.Cities`))
  (for _index (range 1 (+ (`self.NumberOfCities`) 1))
    (bind _returnvalue (`|SpawnActorFromClass` "/Game/Blueprints/City/BP_City.BP_City_C" (`KismetMathLibrary.MakeTransform` (`KismetMathLibrary.MakeVector` (`KismetMathLibrary.RandomFloatInRange` (* -1 _maxrandomx) _maxrandomx) (`KismetMathLibrary.RandomFloatInRange` (* -1 _maxrandomy) _maxrandomy) (`self.CitySpawnHeight`))) "Undefined" "OverrideRootScale" null (`KismetTextLibrary.Conv_IntToText` _index) null))
    (`KismetArrayLibrary.Array_Add` (`self.Cities`) _returnvalue)))

(fn `UserConstructionScript`)